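; Traffic light manager that cycles every BP_TraffictLight1 actor in the level through three colors in sync.
; From BeginPlay, Recolor uses ColorPoint to step through the states, waiting 3, 5 or 1 seconds before setting CurrentColor.
; It then looks up that color in ColorSettings.ColorMap and passes it to each light's ChangeColor.
; The cycle repeats because Recolor calls itself inside a loop over the map's keys.
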(event Custom|Recolor
  (if (== (Variables|Default|GetColorPoint) 0)
    (Utilities|FlowControl|Delay 3.0)
    (Variables|Default|SetCurrentColor "NewEnumerator2")
    (Variables|Default|SetColorPoint (+ (Variables|Default|GetColorPoint) 1))
    (elif (== (Variables|Default|GetColorPoint) 1)
      (Utilities|FlowControl|Delay 5.0)
      (Variables|Default|SetCurrentColor "NewEnumerator1")
      (Variables|Default|SetColorPoint (+ (Variables|Default|GetColorPoint) 1))
      (else
        (Utilities|FlowControl|Delay 1.0)
        (Variables|Default|SetCurrentColor "NewEnumerator0")
        (Variables|Default|SetColorPoint (- (Variables|Default|GetColorPoint) 2)))))
  (bind _outactors (Actor|GetAllActorsOfClass "/Game/Blueprints/BP_TraffictLight1.BP_TraffictLight1_C"))
  (bind _keys (Utilities|Map|Keys (Utilities|Struct|BreakS_LIghtColor (Variables|Default|GetColorSettings))))
  (for _array_element _keys
    (Default|ChangeColor _outactors (.Value (Utilities|Map|Find (Utilities|Struct|BreakS_LIghtColor (Variables|Default|GetColorSettings)) (Variables|Default|GetCurrentColor))))
    (CallFunction|Recolor)))

(event EventBeginPlay
  (CallFunction|Recolor))

(fn ConstructionScript)